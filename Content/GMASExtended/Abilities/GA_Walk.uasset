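; GA_Walk is a GMAS ability that keeps a walk speed effect on its owner while the triggering key is held.
; On begin it applies AE_WalkSpeed as a predicted effect, stores the instance, and waits for key release to end.
; Each tick it also ends itself if the owner has a swimming, crawling or crouching stance tag.
; Ending removes the stored effect through the same predicted queue.
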(event `self.BeginAbilityEvent`
  ;[1 1 1] Apply our speed boost and stamina drain effects.
  (bind (_outsuccess _outeffecthandle _outeffectid _outeffect) (`GMC_AbilitySystemComponent.ApplyAbilityEffectSafe` :`self` (`self.OwnerAbilityComponent`) :`EffectClass` "/Game/GMASExtended/Effects/AE_WalkSpeed.AE_WalkSpeed_C" :`QueueType` "Predicted"))
  (set `self.WalkSpeedEffect` _outeffect)
  ;[1 1 1] Wait for the key which triggered us to be released, then end the ability.
  (`GMCAbilityTask_WaitForInputKeyRelease.WaitForKeyRelease` true
    (:`Completed`
      (`self.EndAbility`))))

(event `self.TickEvent`
  (params (DeltaTime :type "Float (single-precision)"))
  (if (or (`GMC_AbilitySystemComponent.HasActiveTag` (`self.OwnerAbilityComponent`) (struct :`TagName` "Stance.Swimming")) (`GMC_AbilitySystemComponent.HasActiveTag` (`self.OwnerAbilityComponent`) (struct :`TagName` "Stance.Crawling")) (`GMC_AbilitySystemComponent.HasActiveTag` (`self.OwnerAbilityComponent`) (struct :`TagName` "Stance.Crouching")))
    (`self.EndAbility`)))

(event `self.EndAbilityEvent`
  ;[1 1 1] When the ability ends, remove both the speed boost and stamina drain effects.
  (`GMC_AbilitySystemComponent.RemoveActiveAbilityEffectSafe` (`self.OwnerAbilityComponent`) (`self.WalkSpeedEffect`) "Predicted"))