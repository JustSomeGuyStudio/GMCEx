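; GMAS ability for a dive-to-crawl move that plays a montage on the owner pawn's organic movement component.
; It commits the cost if affordable, otherwise ends immediately.
; While the montage plays, a predicted effect grants the State.PlayingMontage tag, which blocks rolling and jumping.
; The ability ends on montage blend-out, and its end event removes the stored effect to clear the tag.
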(event `self.BeginAbilityEvent`
  (if (`self.CanAffordAbilityCost`)
    (`self.CommitAbilityCost`)
    (`|K2Node_PlayMontage` (`Actor.GetComponentByClass` (`self.GetOwnerPawn`) "/Script/GMCExtended.GMCE_OrganicMovementCmp")
      (:`then`
        ;[1 1 1] We will also set the "Play Montage" ability effect. If you look at AE_State_PlayMontage in the Effects directory, you'll see it only sets the State.PlayingMontage tag. Rolling and jumping are blocked by the presence of this tag so that you cannot keep rolling endlessly when already rolling, or jump mid-roll.
        ;
        ; When the ability ends, we remove the effect (and thus the tag).
        (bind (_outsuccess _outeffecthandle _outeffectid _outeffect) (`GMC_AbilitySystemComponent.ApplyAbilityEffectSafe` :`self` (`self.OwnerAbilityComponent`) :`EffectClass` "/Game/GMASExtended/Effects/AE_StatePlayMontage.AE_StatePlayMontage_C" :`QueueType` "Predicted"))
        (set `self.AppliedAbilityEffect` _outeffect))
      (:`OnBlendOut`
        ;[1 1 1] When the montage finishes, end our ability.
        (`self.EndAbility`)))
    (else
      (`self.EndAbility`))))

(event `self.EndAbilityEvent`
  (bind _appliedabilityeffect (`self.AppliedAbilityEffect`))
  (`/Engine/EditorBlueprintResources/StandardMacros.IsValid` _appliedabilityeffect
    (:`Is Valid`
      ;[1 1 1] If we have a stored ability effect, remove it.
      (`GMC_AbilitySystemComponent.RemoveActiveAbilityEffect` (`self.OwnerAbilityComponent`) _appliedabilityeffect))))