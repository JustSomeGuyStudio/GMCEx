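; GA_Jump is a GMAS ability that makes the owning pawn jump with a vertical velocity-change impulse.
; On begin, it commits the ability cost if affordable, applies the impulse and ends; otherwise it just ends.
; The impulse sits just above the organic movement component's MaxGroundedVelocityZ to break grounding.
; If that cast fails, it uses a fixed strength, though still applies it through a GMCE_OrganicMovementCmp lookup.
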(event `self.BeginAbilityEvent`
  (bind _returnvalue (`Actor.GetComponentByClass` (`self.GetOwnerPawn`) "/Script/GMCExtended.GMCE_OrganicMovementCmp"))
  (if (`self.CanAffordAbilityCost`)
    (`self.CommitAbilityCost`)
    (bind _asgmcextended_organic_movement_component (cast `GMCE_OrganicMovementCmp` (`GMC_AbilitySystemComponent.GMCMovementComponent` (`self.OwnerAbilityComponent`)))
      (:`then`
        ;[1 1 1] Add an impulse that is just over our maximum grounded vertical impulse, so that we jump.
        (`GMC_MovementUtilityCmp.AddImpulse` _returnvalue (`KismetMathLibrary.MakeVector` 0.0 0.0 (+ (`GMC_OrganicMovementCmp.MaxGroundedVelocityZ` _asgmcextended_organic_movement_component) 1.0)) true)
        (`self.EndAbility`))
      (:`CastFailed`
        ;[1 1 1] We don't have a valid organic movement component, just use a default jump strength.
        (`GMC_MovementUtilityCmp.AddImpulse` _returnvalue (0.0 0.0 801.0) true)
        (`self.EndAbility`)))
    (else
      (`self.EndAbility`))))