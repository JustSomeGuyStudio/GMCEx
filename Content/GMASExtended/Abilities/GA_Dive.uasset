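; GA_Dive is a GMAS ability for diving that stays active only while the owning pawn is swimming.
; On begin and on every tick, it asks the pawn's GMCE organic movement component whether it is swimming, and ends itself if not.
; The graph applies no dive movement or effects itself, and its end event is empty.
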(event `self.BeginAbilityEvent`
  (if (not (`NavMovementInterface.IsSwimming` (`Actor.GetComponentByClass` (`self.GetOwnerPawn`) "/Script/GMCExtended.GMCE_OrganicMovementCmp")))
    (`self.EndAbility`)))

(event `self.TickEvent`
  (params (DeltaTime :type "Float (single-precision)"))
  (set `self.DeltaTime` DeltaTime)
  (if (not (`NavMovementInterface.IsSwimming` (`Actor.GetComponentByClass` (`self.GetOwnerPawn`) "/Script/GMCExtended.GMCE_OrganicMovementCmp")))
    (`self.EndAbility`)))

(event `self.EndAbilityEvent`)