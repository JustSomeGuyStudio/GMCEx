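; GMAS ability that dashes a swimming pawn forward, requiring horizontal movement and enough stamina.
; On begin it plays a montage, predictively applies montage-state, speed and stamina effects, pushes velocity and impulse along actor forward, and deducts Stamina directly.
; Montage blend-out ends the ability, as does Tick when swimming stops, and ending removes the stored effects.
; CommitAbilityCost is never run, though affordability is checked.
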(event `self.BeginAbilityEvent`
  (bind _returnvalue (`self.GetOwnerPawn`))
  (bind _ownerabilitycomponent (`self.OwnerAbilityComponent`))
  (bind (_returnvalue_x _returnvalue_y) (`KismetMathLibrary.BreakVector` (`GMC_ReplicationCmp.GetLinearVelocity_GMC` (`self.GetOwnerMovementComponent`))))
  (bind _returnvalue_2 (`Actor.GetComponentByClass` _returnvalue "/Script/GMCExtended.GMCE_OrganicMovementCmp"))
  (bind _returnvalue_3 (* (`Actor.GetActorForwardVector` _returnvalue) 1200.0))
  (if (`self.CanAffordAbilityCost`)
    (if (`NavMovementInterface.IsSwimming` (`Actor.GetComponentByClass` (`self.GetOwnerPawn`) "/Script/GMCExtended.GMCE_OrganicMovementCmp"))
      (if (and (> (`GMC_AbilitySystemComponent.GetAttributeValueByTag` (`self.OwnerAbilityComponent`) (struct :`TagName` "Attribute.Stamina")) 5.0) (not (`KismetMathLibrary.Vector_IsNearlyZero` (`KismetMathLibrary.MakeVector` _returnvalue_x _returnvalue_y))))
        (`|K2Node_PlayMontage` (`Actor.GetComponentByClass` (`self.GetOwnerPawn`) "/Script/GMCExtended.GMCE_OrganicMovementCmp")
          (:`then`
            ;[1 1 1] We will also set the "Play Montage" ability effect. If you look at AE_State_PlayMontage in the Effects directory, you'll see it only sets the State.PlayingMontage tag. Rolling and jumping are blocked by the presence of this tag so that you cannot keep rolling endlessly when already rolling, or jump mid-roll.
            ;
            ; When the ability ends, we remove the effect (and thus the tag).
            (bind (_outsuccess _outeffecthandle _outeffectid _outeffect) (`GMC_AbilitySystemComponent.ApplyAbilityEffectSafe` :`self` _ownerabilitycomponent :`EffectClass` "/Game/GMASExtended/Effects/AE_StatePlayMontage.AE_StatePlayMontage_C" :`QueueType` "Predicted"))
            (set `self.AppliedAbilityEffect` _outeffect)
            (bind (_outsuccess_2 _outeffecthandle_2 _outeffectid_2 _outeffect_2) (`GMC_AbilitySystemComponent.ApplyAbilityEffectSafe` :`self` _ownerabilitycomponent :`EffectClass` "/Game/GMASExtended/Effects/AE_SwimDashSpeed.AE_SwimDashSpeed_C" :`QueueType` "Predicted"))
            (set `self.AppliedAbilityEffect_2` _outeffect_2)
            (bind (_outsuccess_3 _outeffecthandle_3 _outeffectid_3 _outeffect_3) (`GMC_AbilitySystemComponent.ApplyAbilityEffectSafe` :`self` _ownerabilitycomponent :`EffectClass` "/Game/GMASExtended/Effects/AE_SwimDashStamina.AE_SwimDashStamina_C" :`QueueType` "Predicted"))
            (set `self.StaminaCostEffect` _outeffect_3)
            (`GMC_MovementUtilityCmp.UpdateVelocity` _returnvalue_2 _returnvalue_3 (`self.DeltaTime`))
            (`GMC_MovementUtilityCmp.AddImpulse` _returnvalue_2 _returnvalue_3 false)
            (`GMC_AbilitySystemComponent.SetAttributeValueByTag` (`self.OwnerAbilityComponent`) (struct :`TagName` "Attribute.Stamina") (- (`GMC_AbilitySystemComponent.GetAttributeValueByTag` (`self.OwnerAbilityComponent`) (struct :`TagName` "Attribute.Stamina")) 1.0) false))
          (:`OnBlendOut`
            ;[1 1 1] When the montage finishes, end our ability.
            (`self.EndAbility`))))
      (else
        (`self.EndAbility`)))
    (else
      (`self.EndAbility`))))

(event `self.EndAbilityEvent`
  (bind _ownerabilitycomponent (`self.OwnerAbilityComponent`))
  (bind _appliedabilityeffect (`self.AppliedAbilityEffect`))
  (`/Engine/EditorBlueprintResources/StandardMacros.IsValid` _appliedabilityeffect
    (:`Is Valid`
      ;[1 1 1] If we have a stored ability effect, remove it.
      (`GMC_AbilitySystemComponent.RemoveActiveAbilityEffect` (`self.OwnerAbilityComponent`) _appliedabilityeffect)
      (`GMC_AbilitySystemComponent.RemoveActiveAbilityEffectSafe` _ownerabilitycomponent (`self.StaminaCostEffect`) "Predicted")
      (`GMC_AbilitySystemComponent.RemoveActiveAbilityEffectSafe` _ownerabilitycomponent (`self.AppliedAbilityEffect`) "Predicted")
      (`GMC_AbilitySystemComponent.RemoveActiveAbilityEffectSafe` _ownerabilitycomponent (`self.AppliedAbilityEffect_2`) "Predicted"))))

(event `self.TickEvent`
  (params (DeltaTime :type "Float (single-precision)"))
  (bind _returnvalue (`Actor.GetComponentByClass` (`self.GetOwnerPawn`) "/Script/GMCExtended.GMCE_OrganicMovementCmp"))
  (set `self.DeltaTime` DeltaTime)
  (if (not (`NavMovementInterface.IsSwimming` (`Actor.GetComponentByClass` (`self.GetOwnerPawn`) "/Script/GMCExtended.GMCE_OrganicMovementCmp")))
    (`GMC_MovementUtilityCmp.StopMontage` _returnvalue (`GMC_OrganicMovementCmp.GetSkeletalMeshReference` _returnvalue) (`GMC_OrganicMovementCmp.MontageTracker` _returnvalue) 0.1)
    (`self.EndAbility`)))