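; GMAS ability that puts its owner into ragdoll while the ability key is held.
; On begin it casts the owner's GMC movement component to GMCE_OrganicMovementCmp, enables ragdoll and waits for key release to end, ending immediately if the cast fails.
; On end it disables ragdoll on the cached component if it is still valid.
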(event `self.BeginAbilityEvent`
  (bind _asgmcextended_organic_movement_component (cast `GMCE_OrganicMovementCmp` (`GMC_AbilitySystemComponent.GMCMovementComponent` (`self.OwnerAbilityComponent`)))
    (:`then`
      (bind _output_get (set `self.GMCE_Component` _asgmcextended_organic_movement_component))
      (`GMCE_OrganicMovementCmp.EnableRagdoll` _output_get)
      (`GMCAbilityTask_WaitForInputKeyRelease.WaitForKeyRelease` true
        (:`Completed`
          (`self.EndAbility`))))
    (:`CastFailed`
      (`self.EndAbility`))))

(event `self.EndAbilityEvent`
  (bind _gmce_component (`self.GMCE_Component`))
  (`/Engine/EditorBlueprintResources/StandardMacros.IsValid` _gmce_component
    (:`Is Valid`
      (`GMCE_OrganicMovementCmp.DisableRagdoll` _gmce_component))))