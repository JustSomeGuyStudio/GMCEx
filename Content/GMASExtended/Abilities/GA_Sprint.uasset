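; GMAS sprint ability that boosts movement speed while draining stamina.
; On begin it requires movement, enough stamina and no crouch or crawl, then sets IsSprinting on BP_ExampleMovement and applies predicted speed and stamina effects.
; It ends on key release, or when Tick detects empty stamina, airborne, montage, crouch or crawl states, removing both effects and clearing the flag.
; A forward-direction check exists but is disconnected.
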(event `self.BeginAbilityEvent`
  (bind _ownerabilitycomponent (`self.OwnerAbilityComponent`))
  (bind (_returnvalue_x _returnvalue_y) (`KismetMathLibrary.BreakVector` (`GMC_ReplicationCmp.GetLinearVelocity_GMC` (`self.GetOwnerMovementComponent`))))
  (bind _asgmcextended_organic_movement_component (cast `GMCE_OrganicMovementCmp` (`GMC_AbilitySystemComponent.GMCMovementComponent` (`self.OwnerAbilityComponent`))))
  (set `self.GMCEMovement` _asgmcextended_organic_movement_component)
  (bind _asbp_example_movement (cast `/Game/GMASExtended/Blueprints/BP_ExampleMovement` _asgmcextended_organic_movement_component))
  (set `self.As BP Example Movement` _asbp_example_movement)
  (if (`KismetMathLibrary.BooleanNOR` (`GMC_AbilitySystemComponent.HasActiveTag` (`self.OwnerAbilityComponent`) (struct :`TagName` "Stance.Crouching")) (`GMC_AbilitySystemComponent.HasActiveTag` (`self.OwnerAbilityComponent`) (struct :`TagName` "Stance.Crawling")))
    (if (and (> (`GMC_AbilitySystemComponent.GetAttributeValueByTag` (`self.OwnerAbilityComponent`) (struct :`TagName` "Attribute.Stamina")) 10.0) (not (`KismetMathLibrary.Vector_IsNearlyZero` (`KismetMathLibrary.MakeVector` _returnvalue_x _returnvalue_y))))
      (set `/Game/GMASExtended/Blueprints/BP_ExampleMovement.IsSprinting` true (`self.As BP Example Movement`))
      ;[1 1 1] Apply our speed boost and stamina drain effects.
      (bind (_outsuccess _outeffecthandle _outeffectid _outeffect) (`GMC_AbilitySystemComponent.ApplyAbilityEffectSafe` :`self` _ownerabilitycomponent :`EffectClass` "/Game/GMASExtended/Effects/AE_SprintSpeed.AE_SprintSpeed_C" :`QueueType` "Predicted"))
      (set `self.SprintSpeedEffect` _outeffect)
      (bind (_outsuccess_2 _outeffecthandle_2 _outeffectid_2 _outeffect_2) (`GMC_AbilitySystemComponent.ApplyAbilityEffectSafe` :`self` _ownerabilitycomponent :`EffectClass` "/Game/GMASExtended/Effects/AE_SprintStamina.AE_SprintStamina_C" :`QueueType` "Predicted"))
      (set `self.StaminaCostEffect` _outeffect_2)
      ;[1 1 1] Wait for the key which triggered us to be released, then end the ability.
      (`GMCAbilityTask_WaitForInputKeyRelease.WaitForKeyRelease` true
        (:`Completed`
          (`self.EndAbility`)))
      (else
        (`self.EndAbility`)))
    (else
      (`self.EndAbility`))))

(event `self.TickEvent`
  (params (DeltaTime :type "Float (single-precision)"))
  (bind _ownerabilitycomponent (`self.OwnerAbilityComponent`))
  ;[1 1 1] If we've run out of stamina, end our ability.
  (if (or (<= (`GMC_AbilitySystemComponent.GetAttributeValueByTag` (`self.OwnerAbilityComponent`) (struct :`TagName` "Attribute.Stamina")) 0.0) (`ActorComponent.ComponentHasTag` _ownerabilitycomponent "State.InAir") (`ActorComponent.ComponentHasTag` _ownerabilitycomponent "State.PlayingMontage") (`GMC_AbilitySystemComponent.HasActiveTag` (`self.OwnerAbilityComponent`) (struct :`TagName` "Stance.Crouching")) (`GMC_AbilitySystemComponent.HasActiveTag` (`self.OwnerAbilityComponent`) (struct :`TagName` "Stance.Crawling")))
    (`self.EndAbility`)))

(event `self.EndAbilityEvent`
  (bind _ownerabilitycomponent (`self.OwnerAbilityComponent`))
  ;[1 1 1] When the ability ends, remove both the speed boost and stamina drain effects.
  (`GMC_AbilitySystemComponent.RemoveActiveAbilityEffectSafe` _ownerabilitycomponent (`self.StaminaCostEffect`) "Predicted")
  (`GMC_AbilitySystemComponent.RemoveActiveAbilityEffectSafe` _ownerabilitycomponent (`self.SprintSpeedEffect`) "Predicted")
  (set `/Game/GMASExtended/Blueprints/BP_ExampleMovement.IsSprinting` false (`self.As BP Example Movement`)))