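; Example first-person pawn for GMAS that routes player input to abilities and shows status effects on other players' pawns.
; BeginPlay adds the HUD widget, and Jump, Roll and Sprint inputs queue tagged abilities, with Sprint skipped while already sprinting.
; Every tick, non-locally controlled pawns with the Burning tag get a Niagara aura and overlay material, styled by the Healing tag.
; The overlay's dynamic material instance is recreated each tick while active.
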(event `self.ReceiveBeginPlay`
  (bind _asgmc_player_controller (cast `GMC_PlayerController` (`GameplayStatics.GetPlayerControllerFromID` 0)))
  (bind _returnvalue (`|CreateWidget` "/Game/GMASExtended/UI/WBP_HUD.WBP_HUD_C" _asgmc_player_controller))
  (`UserWidget.AddToViewport` _returnvalue 0))

(event `self.ReceiveTick`
  (params (DeltaSeconds :type "Float (single-precision)"))
  (`parent.ReceiveTick` DeltaSeconds)
  (`self.ShowStatusEffects`))

(event `EnhancedInput|/Game/GMASExtended/Input/IA_Jump`
  (params (ActionValue :type Boolean) (ElapsedSeconds :type "Float (double-precision)") (TriggeredSeconds :type "Float (double-precision)") (InputAction :type "InputAction Object Reference" :default "/Game/GMASExtended/Input/IA_Jump.IA_Jump"))
  (:`Triggered`
    (`GMC_AbilitySystemComponent.QueueAbility` (`self.AbilitySystemComponent`) (struct :`TagName` "Ability.Jump") InputAction)))

(event `EnhancedInput|/Game/GMASExtended/Input/IA_Roll`
  (params (ActionValue :type Boolean) (ElapsedSeconds :type "Float (double-precision)") (TriggeredSeconds :type "Float (double-precision)") (InputAction :type "InputAction Object Reference" :default "/Game/GMASExtended/Input/IA_Roll.IA_Roll"))
  (:`Triggered`
    (`GMC_AbilitySystemComponent.QueueAbility` (`self.AbilitySystemComponent`) (struct :`TagName` "Ability.Roll") InputAction)))

(event `EnhancedInput|/Game/GMASExtended/Input/IA_Sprint`
  (params (ActionValue :type Boolean) (ElapsedSeconds :type "Float (double-precision)") (TriggeredSeconds :type "Float (double-precision)") (InputAction :type "InputAction Object Reference" :default "/Game/GMASExtended/Input/IA_Sprint.IA_Sprint"))
  (bind _abilitysystemcomponent (`self.AbilitySystemComponent`))
  (:`Started`
    (if (not (`GMC_AbilitySystemComponent.HasAnyTagExact` _abilitysystemcomponent (struct :`GameplayTags` (struct :`(TagName` "Buff.Sprinting")))))
      (`GMC_AbilitySystemComponent.QueueAbility` _abilitysystemcomponent (struct :`TagName` "Ability.Sprint") InputAction))))

(fn `ShowStatusEffects`
  (bind _skeletalmesh (`self.SkeletalMesh`))
  (bind _status_aura (`self.Status_Aura`))
  (bind _returnvalue (`GMC_AbilitySystemComponent.HasActiveTag` (`self.AbilitySystemComponent`) (struct :`TagName` "State.Healing")))
  (bind _returnvalue_2 (`KismetMathLibrary.SelectColor` (struct :`G` 200.0 :`A` 1.0) (struct :`R` 0.855903 :`A` 1.0) _returnvalue))
  (if (`self.IsLocallyControlled`)
    _
    (elif (`GMC_AbilitySystemComponent.HasAnyTag` (`self.AbilitySystemComponent`) (struct :`GameplayTags` (struct :`(TagName` "State.Burning") :`(TagName` "State.Healing"))))
      (`NiagaraComponent.SetVariableLinearColor` _status_aura "Color" _returnvalue_2)
      (`NiagaraComponent.SetVariableFloat` _status_aura "SpawnRate" (`KismetMathLibrary.SelectFloat` 0.0 120.0 _returnvalue))
      (`NiagaraComponent.SetVariableBool` _status_aura "UseOrbiters" _returnvalue)
      (`NiagaraFunctionLibrary.OverrideSystemUserVariableSkeletalMeshComponent` _status_aura "" _skeletalmesh)
      (`ActorComponent.Activate` _status_aura false)
      (bind _returnvalue_3 (`KismetMaterialLibrary.CreateDynamicMaterialInstance` "/Game/GMASExtended/Particles/M_Aura_Overlay.M_Aura_Overlay" "None" "Transient"))
      (`MaterialInstanceDynamic.SetVectorParameterValue` _returnvalue_3 "Color" _returnvalue_2)
      (`MeshComponent.SetOverlayMaterial` _skeletalmesh _returnvalue_3)
      (else
        (`ActorComponent.Deactivate` (`self.Status_Aura`))
        (`MeshComponent.SetOverlayMaterial` (`self.SkeletalMesh`) null)))))

(fn `UserConstructionScript`)