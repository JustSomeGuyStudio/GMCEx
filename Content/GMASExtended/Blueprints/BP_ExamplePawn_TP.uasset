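; Third-person example pawn that routes input to gameplay abilities and handles HUD, death and respawn.
; Jump, roll, sprint and ragdoll input queue abilities by tag; jump respawns when dead.
; Health reaching zero triggers ragdoll and a local respawn widget, while respawning restores health and stamina.
; Tick drives a burning-gated Niagara aura and overlay, varied by healing, and optionally blends camera presets for aim, strafe or default.
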(event `self.ReceiveBeginPlay`
  (add `GMC_AbilitySystemComponent.OnAttributeChanged` (`self.AbilitySystemComponent`) (delegate `OnAttributeChanged`))
  (`self.Setup`)
  (if (`self.AutomaticCameraEnable`)
    (`self.SetCameraByState`)
    (`self.UpdateCamera` false)))

(event `EnhancedInput|/Game/GMASExtended/Input/IA_Jump`
  (params (ActionValue :type Boolean) (ElapsedSeconds :type "Float (double-precision)") (TriggeredSeconds :type "Float (double-precision)") (InputAction :type "InputAction Object Reference" :default "/Game/GMASExtended/Input/IA_Jump.IA_Jump"))
  (:`Started`
    (`self.HandleJump` InputAction)))

(event `OnAttributeChanged`
  (params (AttributeTag :type "GameplayTag Structure") (OldValue :type "Float (single-precision)") (NewValue :type "Float (single-precision)"))
  (if (and (== AttributeTag (struct :`TagName` "Attribute.Health")) (> OldValue 0.0) (<= NewValue 0.0))
    (`self.HandleDeath`)))

(event `EnhancedInput|/Game/GMASExtended/Input/IA_Roll`
  (params (ActionValue :type Boolean) (ElapsedSeconds :type "Float (double-precision)") (TriggeredSeconds :type "Float (double-precision)") (InputAction :type "InputAction Object Reference" :default "/Game/GMASExtended/Input/IA_Roll.IA_Roll"))
  (:`Triggered`
    (`GMC_AbilitySystemComponent.QueueAbility` (`self.AbilitySystemComponent`) (struct :`TagName` "Ability.Roll") InputAction)))

(event `self.ReceiveTick`
  (params (DeltaSeconds :type "Float (single-precision)"))
  (`parent.ReceiveTick` DeltaSeconds)
  (`self.ShowStatusEffects`)
  (if (`self.AutomaticCameraEnable`)
    (`self.SetCameraByState`)
    (`self.UpdateCamera` true)))

(event `EnhancedInput|/Game/GMASExtended/Input/IA_Sprint`
  (params (ActionValue :type Boolean) (ElapsedSeconds :type "Float (double-precision)") (TriggeredSeconds :type "Float (double-precision)") (InputAction :type "InputAction Object Reference" :default "/Game/GMASExtended/Input/IA_Sprint.IA_Sprint"))
  (bind _abilitysystemcomponent (`self.AbilitySystemComponent`))
  (:`Started`
    (if (not (`GMC_AbilitySystemComponent.HasAnyTagExact` _abilitysystemcomponent (struct :`GameplayTags` (struct :`(TagName` "Buff.Sprinting")))))
      (`GMC_AbilitySystemComponent.QueueAbility` _abilitysystemcomponent (struct :`TagName` "Ability.Sprint") InputAction))))

(event `EnhancedInput|/Game/GMASExtended/Input/IA_Ragdoll`
  (params (ActionValue :type Boolean) (ElapsedSeconds :type "Float (double-precision)") (TriggeredSeconds :type "Float (double-precision)") (InputAction :type "InputAction Object Reference" :default "/Game/GMASExtended/Input/IA_Ragdoll.IA_Ragdoll"))
  (:`Triggered`
    (`GMC_AbilitySystemComponent.QueueAbility` (`self.AbilitySystemComponent`) (struct :`TagName` "Ability.Ragdoll") InputAction)))

(event `self.OnRespawn`
  (bind _abilitysystemcomponent (`self.AbilitySystemComponent`))
  (bind _respawnwidget (`self.RespawnWidget`))
  (bind _abilitysystemcomponent_2 (`self.AbilitySystemComponent`))
  (`GMCE_OrganicMovementCmp.DisableRagdoll` (`self.Template Movement Component`))
  ;[0.1188 1 0.1619] Reset health and stamina attributes to max values.
  (`GMC_AbilitySystemComponent.SetAttributeValueByTag` _abilitysystemcomponent (struct :`TagName` "Attribute.Health") (`GMC_AbilitySystemComponent.GetAttributeValueByTag` _abilitysystemcomponent_2 (struct :`TagName` "Attribute.HealthMax")) true)
  (`GMC_AbilitySystemComponent.SetAttributeValueByTag` _abilitysystemcomponent (struct :`TagName` "Attribute.Stamina") (`GMC_AbilitySystemComponent.GetAttributeValueByTag` _abilitysystemcomponent_2 (struct :`TagName` "Attribute.StaminaMax")) true)
  ;[1 0.05949 0.7813] Remove the respawn overlay widget (if we have one).
  (`/Engine/EditorBlueprintResources/StandardMacros.IsValid` _respawnwidget
    (:`Is Valid`
      (`Widget.RemoveFromParent` _respawnwidget)
      (set `self.RespawnWidget` null))))

(fn `HandleDeath`
  (`GMC_AbilitySystemComponent.AddActiveTag` (`self.AbilitySystemComponent`) (struct :`TagName` "State.Dead"))
  (`GMCE_OrganicMovementCmp.EnableRagdoll` (`self.Template Movement Component`))
  (if (and (`self.IsLocallyControlled`) (not (`KismetSystemLibrary.IsValid` (`self.RespawnWidget`))))
    (bind _returnvalue (`|CreateWidget` "/Game/GMASExtended/UI/WBP_Respawn.WBP_Respawn_C" (`GameplayStatics.GetPlayerControllerFromID` 0)))
    (bind _output_get (set `self.RespawnWidget` _returnvalue))
    (`UserWidget.AddToViewport` _output_get 1)))

(fn `HandleJump`
  (params (InputAction :type "InputAction Object Reference"))
  (if (`GMC_AbilitySystemComponent.HasActiveTag` (`self.AbilitySystemComponent`) (struct :`TagName` "State.Dead"))
    (`self.Respawn`)
    (else
      (`GMC_AbilitySystemComponent.QueueAbility` (`self.AbilitySystemComponent`) (struct :`TagName` "Ability.Jump") InputAction))))

(fn `SetCameraByState`
  (bind _abilitysystemcomponent (`self.AbilitySystemComponent`))
  (if (`GMC_AbilitySystemComponent.HasActiveTag` _abilitysystemcomponent (struct :`TagName` "State.IsAiming"))
    (set `self.ActiveCameraSettings` (`self.Camera_Aim`))
    (elif (`GMC_AbilitySystemComponent.HasActiveTag` _abilitysystemcomponent (struct :`TagName` "State.IsStrafing"))
      (set `self.ActiveCameraSettings` (`self.Camera_Strafe`))
      (else
        (set `self.ActiveCameraSettings` (`self.Camera_Default`))))))

(fn `Setup`
  (bind _asgmc_player_controller (cast `GMC_PlayerController` (`GameplayStatics.GetPlayerControllerFromID` 0)))
  (bind _returnvalue (`|CreateWidget` "/Game/GMASExtended/UI/WBP_HUD.WBP_HUD_C" _asgmc_player_controller))
  (bind _output_get (set `self.StatusWidget` _returnvalue))
  (`UserWidget.AddToViewport` _returnvalue 0)
  (`UserWidget.AddToViewport` _output_get 0))

(fn `ShowStatusEffects`
  (bind _status_aura (`self.Status_Aura`))
  (bind _status_aura_2 (`self.Status_Aura`))
  (bind _returnvalue (`GMC_AbilitySystemComponent.HasActiveTag` (`self.AbilitySystemComponent`) (struct :`TagName` "State.Healing")))
  (bind _returnvalue_2 (`KismetMathLibrary.SelectColor` (struct :`G` 0.630208 :`A` 1.0) (struct :`R` 0.855903 :`A` 1.0) _returnvalue))
  (if (`GMC_AbilitySystemComponent.HasAnyTag` (`self.AbilitySystemComponent`) (struct :`GameplayTags` (struct :`(TagName` "State.Burning") :`(TagName` "State.Healing"))))
    (if (!= (`self.HasHealAura`) _returnvalue)
      (`NiagaraComponent.ResetSystem` (`self.Status_Aura`)))
    (set `self.HasHealAura` _returnvalue)
    ;[0.2793 0.3872 0.1097] Set up particle system and overlay material
    (`NiagaraComponent.SetVariableLinearColor` _status_aura "Color" _returnvalue_2)
    (`NiagaraComponent.SetVariableFloat` _status_aura "SpawnRate" (`KismetMathLibrary.SelectFloat` 0.0 120.0 _returnvalue))
    (`NiagaraComponent.SetVariableBool` _status_aura "UseOrbiters" _returnvalue)
    (`NiagaraFunctionLibrary.OverrideSystemUserVariableSkeletalMeshComponent` _status_aura "" (`self.MeshComponent`))
    (`NiagaraComponent.SetVariableBool` _status_aura "UseFlames" (not (`self.HasHealAura`)))
    (`ActorComponent.Activate` _status_aura false)
    (bind _returnvalue_3 (`KismetMaterialLibrary.CreateDynamicMaterialInstance` "/Game/GMASExtended/Particles/M_Aura_Overlay.M_Aura_Overlay" "None" "Transient"))
    (`MaterialInstanceDynamic.SetVectorParameterValue` _returnvalue_3 "Color" _returnvalue_2)
    (`MeshComponent.SetOverlayMaterial` (`self.MeshComponent`) _returnvalue_3)
    (else
      (`NiagaraComponent.SetVariableBool` _status_aura_2 "UseFlames" false)
      (`NiagaraComponent.SetVariableBool` _status_aura_2 "UseOrbiters" false)
      (`ActorComponent.Deactivate` _status_aura_2)
      (`MeshComponent.SetOverlayMaterial` (`self.MeshComponent`) null))))

(fn `UpdateCamera`
  (params (Interpolate :type Boolean))
  (locals (TemporaryCameraSettings :type "/Game/GMASExtended/Data/S_CameraParameters Structure"))
  (bind (_activecamerasettings_springarmlength _activecamerasettings_fieldofview _activecamerasettings_transitionspeed _activecamerasettings_socketoffset _activecamerasettings_translationlagspeed) (break `/Game/GMASExtended/Data/S_CameraParameters` (`self.ActiveCameraSettings`)))
  (bind (_temporarycamerasettings_springarmlength _temporarycamerasettings_fieldofview _temporarycamerasettings_transitionspeed) (break `/Game/GMASExtended/Data/S_CameraParameters` (`local.TemporaryCameraSettings`)))
  (bind (_temporarycamerasettings_springarmlength_2 _temporarycamerasettings_fieldofview_2 _temporarycamerasettings_transitionspeed_2 _temporarycamerasettings_socketoffset) (break `/Game/GMASExtended/Data/S_CameraParameters` (`local.TemporaryCameraSettings`)))
  (bind (_temporarycamerasettings_springarmlength_3 _temporarycamerasettings_fieldofview_3 _temporarycamerasettings_transitionspeed_3 _temporarycamerasettings_socketoffset_2 _temporarycamerasettings_translationlagspeed) (break `/Game/GMASExtended/Data/S_CameraParameters` (`local.TemporaryCameraSettings`)))
  (bind _interpolate (`local.Interpolate`))
  (bind (_temporarycamerasettings_springarmlength_4 _temporarycamerasettings_fieldofview_4 _temporarycamerasettings_transitionspeed_4) (break `/Game/GMASExtended/Data/S_CameraParameters` (`local.TemporaryCameraSettings`)))
  (set `local.TemporaryCameraSettings` (make `/Game/GMASExtended/Data/S_CameraParameters` _activecamerasettings_springarmlength _activecamerasettings_fieldofview (`KismetMathLibrary.SelectFloat` _activecamerasettings_transitionspeed -1.0 _interpolate) _activecamerasettings_socketoffset (`KismetMathLibrary.SelectFloat` _activecamerasettings_translationlagspeed -1.0 _interpolate)))
  (bind _output_get (set `CameraComponent.FieldOfView` (`KismetMathLibrary.FInterpTo` (stale _output_get) _temporarycamerasettings_fieldofview_4 (`GameplayStatics.GetWorldDeltaSeconds`) _temporarycamerasettings_transitionspeed_4) (`self.CameraComponent`)))
  (bind _output_get_2 (set `SpringArmComponent.TargetArmLength` (`KismetMathLibrary.FInterpTo` (stale _output_get_2) _temporarycamerasettings_springarmlength (`GameplayStatics.GetWorldDeltaSeconds`) _temporarycamerasettings_transitionspeed) (`self.SpringArmComponent`)))
  (bind _output_get_3 (set `SpringArmComponent.SocketOffset` (`KismetMathLibrary.VInterpTo` (stale _output_get_3) _temporarycamerasettings_socketoffset (`GameplayStatics.GetWorldDeltaSeconds`) _temporarycamerasettings_transitionspeed_2) (`self.SpringArmComponent`)))
  (bind _output_get_4 (set `SpringArmComponent.CameraLagSpeed` (`KismetMathLibrary.FInterpTo` (stale _output_get_4) _temporarycamerasettings_translationlagspeed (`GameplayStatics.GetWorldDeltaSeconds`) _temporarycamerasettings_transitionspeed_3) (`self.SpringArmComponent`))))

(fn `UserConstructionScript`)